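; BP_EQControler is an audio visualizer that scales a set of actors like equalizer bars.
; Each Tick it calculates the frequency spectrum of a short window of the Track sound wave, starting at the current game time, with one band per entry in Actors.
; Each actor's Z scale follows the scaled absolute value of its band.
; The Blueprint never plays the track, so analysis follows game time rather than playback position.
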(event `self.ReceiveBeginPlay`)

(event `self.ReceiveTick`
  (params (DeltaSeconds :type "Float (single-precision)"))
  (bind _outspectrum (`SoundVisualizationStatics.CalculateFrequencySpectrum` (`self.Track`) 0 (`KismetSystemLibrary.GetGameTimeInSeconds`) 0.1 (`KismetArrayLibrary.Array_Length` (`self.Actors`))))
  (set `self.Spectrum` _outspectrum)
  (for (_array_element _array_index) (`self.Actors`)
    (`self.SetActorScale3D` _array_element (`KismetMathLibrary.MakeVector` 1.0 1.0 (* (`KismetMathLibrary.Abs` (`|GetArrayItem` (`self.Spectrum`) _array_index)) 0.1)))))

(fn `UserConstructionScript`)